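; Player state for RGB Box Escaper that tracks health and red, green and blue box counts to decide death and victory.
; Damage is ignored once HP reaches zero, while healing adds a fixed amount clamped to max HP.
; Each box pickup increments a count capped at three, and having all three colors full triggers Win.
; Event dispatchers broadcast HP changes, count updates, death and victory to listeners.
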(fn ConstructionScript)

(fn AddDamage
  (params (Damage :type Float%20%28double-precision%29))
  (if (not (CallFunction|IsDeath))
    (bind _output_get (Variables|Default|SetCurHp (- (Variables|Default|GetCurHp) Damage)))
    (Default|CallEventDispatcherUpdateHp _output_get (Variables|Default|GetMaxHp))
    (if (<= (Variables|Default|GetCurHp) 0.0)
      (Default|CallEventDispatcherDeath))))

(fn IsDeath
  (return (<= (Variables|Default|GetCurHp) 0.0)))

(fn AddHeal
  (bind _output_get (Variables|Default|SetCurHp (Math|Float|Clamp(Float) (+ (Variables|Default|GetCurHp) 1e+01) 0.0 (Variables|Default|GetMaxHp))))
  (Default|CallEventDispatcherUpdateHp _output_get (Variables|Default|GetMaxHp)))

(fn AddRedBoxCount
  (bind _output_get (Variables|Default|SetRedBoxCount (Math|Integer|Clamp(Integer) (+ (Variables|Default|GetRedBoxCount) 1) 0 3)))
  (Default|CallEventDispatcherUpdateBoxCount _output_get (Variables|Default|GetGreenBoxCount) (Variables|Default|GetBlueBoxCount))
  (CallFunction|VictoryCheck))

(fn AddGreenBoxCount
  (bind _output_get (Variables|Default|SetGreenBoxCount (Math|Integer|Clamp(Integer) (+ (Variables|Default|GetGreenBoxCount) 1) 0 3)))
  (Default|CallEventDispatcherUpdateBoxCount (Variables|Default|GetRedBoxCount) _output_get (Variables|Default|GetBlueBoxCount))
  (CallFunction|VictoryCheck))

(fn AddBlueBoxCount
  (bind _output_get (Variables|Default|SetBlueBoxCount (Math|Integer|Clamp(Integer) (+ (Variables|Default|GetBlueBoxCount) 1) 0 3)))
  (Default|CallEventDispatcherUpdateBoxCount (Variables|Default|GetRedBoxCount) (Variables|Default|GetGreenBoxCount) _output_get)
  (CallFunction|VictoryCheck))

(fn VictoryCheck
  (if (Math|Boolean|ANDBoolean (== (Variables|Default|GetRedBoxCount) 3) (== (Variables|Default|GetGreenBoxCount) 3) (== (Variables|Default|GetBlueBoxCount) 3))
    (Default|CallEventDispatcherWin)))