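; Component that keeps up to ten random items spawned on the navmesh around its owner in RGBBoxEscaper.
; Each tick, while the count is below the cap, it picks a random DT_Item row and spawns that row's class at a random navigable point near the owner, passing the row as ItemData.
; Each spawn increments the count, and SubItemCount provides a clamped decrement that lets spawning resume.
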(event EventBeginPlay
  (Variables|Default|SetItemCount 0))

(event EventTick
  (params (DeltaSeconds :type Float%20%28single-precision%29))
  (bind _needitem (CallFunction|CheckItemCount))
  (if _needitem
    (CallFunction|DoSpawnItem)))

(fn DoSpawnItem
  (bind _randomlocation (Class|NavigationSystemV1|GetRandomLocationinNavigableRadius (Transformation|GetActorLocation (Components|GetOwner)) 1e+03 0 0))
  (bind _outrownames (DataTable|GetDataTableRowNames "/Game/RGBBoxEscaper/Items/DT_Item.DT_Item"))
  (bind _returnvalue (Utilities|GetDataTableRow "/Game/RGBBoxEscaper/Items/DT_Item.DT_Item" (.OutItem (Utilities|Array|Random _outrownames)))
    (:then
      (Game|SpawnActorfromClass (.ItemClass (Utilities|Struct|BreakST_Item _returnvalue)) (Math|Transform|MakeTransform _randomlocation "0, 0, 0" "1.000000,1.000000,1.000000") "Undefined" "MultiplyWithRoot" 0 _returnvalue 0)
      (CallFunction|AddItemCount))))

(fn CheckItemCount
  (return (< (Variables|Default|GetItemCount) 10)))

(fn AddItemCount
  (Variables|Default|SetItemCount (+ (Variables|Default|GetItemCount) 1)))

(fn SubItemCount
  (Variables|Default|SetItemCount (Math|Integer|Clamp(Integer) (- (Variables|Default|GetItemCount) 1) 0 10)))